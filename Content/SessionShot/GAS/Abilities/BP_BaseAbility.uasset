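; Base Gameplay Ability Blueprint that provides shared helpers for the game's character abilities.
; On activation it adds a non-replicated AbilityInProgress loose tag to the avatar and removes it when the ability ends.
; Helper functions toggle player input, movement mode and ranged/melee attack permission, create viewport widgets, and run a sphere trace along the player's camera view.
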(event `self.K2_ActivateAbility`
  (bind _returnvalue (`self.GetAvatarActorFromActorInfo`))
  (`/Engine/EditorBlueprintResources/StandardMacros.IsValid` _returnvalue
    (:`Is Valid`
      (`AbilitySystemBlueprintLibrary.AddLooseGameplayTags` _returnvalue (`BlueprintGameplayTagLibrary.MakeGameplayTagContainerFromTag` (struct :`TagName` "Character.State.AbilityInProgress"))))))

(event `self.K2_OnEndAbility`
  (params (bWasCancelled :type Boolean))
  (bind _returnvalue (`self.GetAvatarActorFromActorInfo`))
  (`/Engine/EditorBlueprintResources/StandardMacros.IsValid` _returnvalue
    (:`Is Valid`
      (`AbilitySystemBlueprintLibrary.RemoveLooseGameplayTags` _returnvalue (`BlueprintGameplayTagLibrary.MakeGameplayTagContainerFromTag` (struct :`TagName` "Character.State.AbilityInProgress"))))))

(fn `ChangeInputState`
  (params (InputEnabled :type Boolean))
  (bind _aspawn (cast `Pawn` (`self.GetAvatarActorFromActorInfo`)))
  (bind _asplayer_controller (cast `PlayerController` (`Pawn.GetController` _aspawn)))
  (if InputEnabled
    (`Actor.EnableInput` _asplayer_controller _asplayer_controller)
    (else
      (`Actor.DisableInput` _asplayer_controller _asplayer_controller))))

(fn `ChangeMovementState`
  (params (CanMove :type Boolean))
  (`CharacterMovementComponent.SetMovementMode` (`Actor.GetComponentByClass` (`self.GetAvatarActorFromActorInfo`) "/Script/Engine.CharacterMovementComponent") (select `bool` CanMove :`false` "MOVE_None" :`true` "MOVE_Walking" :!type "EMovementMode Enum") 0))

(fn `CreateWidget`
  (params (Class :type "UserWidget Class Reference") (OwningPlayer :type "PlayerController Object Reference"))
  (returns (ReturnValue :type "UserWidget Object Reference"))
  (bind _returnvalue (`|CreateWidget` Class OwningPlayer))
  (`UserWidget.AddToViewport` _returnvalue 0)
  (return _returnvalue))

(fn `MakeSphereTrace`
  (params (TraceLength :type "Float (single-precision)") (TraceRadius :type "Float (double-precision)") (ActorsToIgnore :type "Array of Actor Object Reference (by ref)"))
  (returns (OutHit :type "HitResult Structure") (ReturnValue :type Boolean))
  (locals (Length :type "Float (single-precision)") (Radius :type "Float (double-precision)") (IgnoredActors :type "Array of Actor Object Reference"))
  (set `local.Length` TraceLength)
  (set `local.Radius` TraceRadius)
  (set `local.IgnoredActors` ActorsToIgnore)
  (bind _aspawn (cast `Pawn` (`self.GetAvatarActorFromActorInfo`))
    (:`then`
      (bind _asplayer_controller (cast `PlayerController` (`Pawn.GetController` _aspawn))
        (:`then`
          (bind (_location _rotation) (`Controller.GetPlayerViewPoint` _asplayer_controller))
          (bind (_outhit _returnvalue) (`KismetSystemLibrary.SphereTraceSingle` _location (+ _location (* (`KismetMathLibrary.Conv_RotatorToVector` _rotation) (`local.Length`))) (`local.Radius`) "TraceTypeQuery1" false (`local.IgnoredActors`)))
          (return _outhit _returnvalue))
        (:`CastFailed`
          _)))
    (:`CastFailed`
      _))
  (return (struct) false))

(fn `SetCanPlayerAttack`
  (params (CanOwnerAttack :type Boolean))
  (bind _returnvalue (`self.GetAvatarActorFromActorInfo`))
  (`/Engine/EditorBlueprintResources/StandardMacros.IsValid` _returnvalue
    (:`Is Valid`
      (`BaseAttackComponent.SetCanOwnerAttack` (`Actor.GetComponentByClass` _returnvalue "/Script/SessionShot.RangeAttackComponent") CanOwnerAttack)
      (`BaseAttackComponent.SetCanOwnerAttack` (`Actor.GetComponentByClass` _returnvalue "/Script/SessionShot.MeleeAttackComponent") CanOwnerAttack))))