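; Gameplay ability for Kallari's ultimate slash, a targeted teleport strike on another player, activatable only while Concentration is non-zero.
; Holding input shows a crosshair to the local player; release runs a sphere trace for a player-class target.
; A hit moves the avatar to the impact point facing the target, then commits the ability, plays the montage and triggers a sword-socket attack through the melee component.
; A miss or failed move ends the ability uncommitted.
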(event `self.K2_ActivateAbility`
  (bind _returnvalue (`self.GetAvatarActorFromActorInfo`))
  (bind (_returnvalue_roll _returnvalue_pitch) (`KismetMathLibrary.BreakRotator` (`Actor.K2_GetActorRotation` _returnvalue)))
  (`AbilityTask_WaitInputRelease.WaitInputRelease` true
    (:`then`
      (`self.IsLocallyControlled`
        (:`True`
          (bind _returnvalue_2 (`self.CreateWidget` (`self.CrosshairClass`)))
          (set `self.CreatedWidget` _returnvalue_2))))
    (:`OnRelease`
      (bind _outhit (`self.MakeSphereTrace` (`self.AbilityTraceLength`) (`self.AbilityTraceRadius`) (`|MakeArray` (`self.GetAvatarActorFromActorInfo`))))
      (if (`GameplayStatics.ObjectIsA` (`.HitActor` (`GameplayStatics.BreakHitResult` _outhit)) (`self.PlayerClass`))
        (bind (_returnvalue_x _returnvalue_y _returnvalue_z) (`KismetMathLibrary.BreakVector` (`Actor.K2_GetActorLocation` (`.HitActor` (`GameplayStatics.BreakHitResult` _outhit)))))
        (bind (_returnvalue_roll_2 _returnvalue_pitch_2 _returnvalue_yaw) (`KismetMathLibrary.BreakRotator` (`KismetMathLibrary.Conv_VectorToRotator` (* (`.ImpactNormal` (`GameplayStatics.BreakHitResult` _outhit)) -1.0))))
        (bind (_sweephitresult _returnvalue_3) (`Actor.K2_SetActorLocationAndRotation` _returnvalue (`KismetMathLibrary.MakeVector` (.x (`.Location` (`GameplayStatics.BreakHitResult` _outhit))) (.y (`.Location` (`GameplayStatics.BreakHitResult` _outhit))) _returnvalue_z) (`KismetMathLibrary.MakeRotator` _returnvalue_roll _returnvalue_pitch _returnvalue_yaw) false false))
        (if _returnvalue_3
          (bind _returnvalue_4 (`self.K2_CommitAbility`))
          (if _returnvalue_4
            (`self.IsLocallyControlled`
              (:`True`
                (`Widget.RemoveFromParent` (`self.CreatedWidget`)))
              (:`False`
                _))
            (`AbilityTask_PlayMontageAndWait.CreatePlayMontageAndWaitProxy` "None" (`self.AttackMontage`) 1.0 "None" false
              (:`then`
                (`MeleeAttackComponent.ExecuteSpecificAttack` (`self.GetCharacterMeleeComponent`) (make `AttackData` (`self.AttackEffect`) 1 null "sword_base_r" "sword_tip_r"))
                (`self.K2_EndAbility`)))
            (else
              (`self.K2_EndAbility`)))
          (else
            (`self.K2_EndAbility` :!label _label)
            (`self.IsLocallyControlled`
              (:`True`
                (`Widget.RemoveFromParent` (`self.CreatedWidget`))))))
        (else
          (goto _label))))))

(fn `GetCharacterMeleeComponent`
  (returns (ReturnValue :type "MeleeAttackComponent Object Reference"))
  (locals (MeleeComponentClass :type "MeleeAttackComponent Class Reference" :default "/Script/CoreUObject.Class'/Script/SessionShot.MeleeAttackComponent'"))
  (return (`Actor.GetComponentByClass` (`self.GetAvatarActorFromActorInfo`) (`local.MeleeComponentClass`))))

(fn `K2_CanActivateAbility`
  (params (ActorInfo :type "GameplayAbilityActorInfo Structure") (Handle :type "GameplayAbilitySpecHandle Structure"))
  (returns (RelevantTags :type "GameplayTagContainer Structure") (ReturnValue :type Boolean))
  (bind (_owneractor _avataractor _playercontroller _abilitysystemcomponent) (break `GameplayAbilityActorInfo` ActorInfo))
  (`/Engine/EditorBlueprintResources/StandardMacros.IsValid` _abilitysystemcomponent
    (:`Is Valid`
      (bind _returnvalue (`AbilitySystemComponent.GetAttributeSet` _abilitysystemcomponent "/Script/GameplayAbilities.AttributeSet"))
      (bind _asbase_attribute_set (cast `BaseAttributeSet` _returnvalue)
        (:`then`
          (return (struct) (not (`KismetMathLibrary.NearlyEqual_FloatFloat` (`BaseAttributeSet.GetConcentrationPercent` _asbase_attribute_set)))))
        (:`CastFailed`
          _)))
    (:`Is Not Valid`
      _))
  (return (struct) false))