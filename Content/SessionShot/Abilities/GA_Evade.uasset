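; Gameplay Ability for an evade that launches the avatar forward or backward with added lift, only activatable when not falling.
; Velocity nearly aligned with the facing vector selects forward; anything else, including standing still, evades backward.
; After commit, it disables player input and applies a constant root motion force alongside the matching directional montage.
; Montage completion, blend-out, interruption or cancellation restores input and ends the ability.
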(event `self.K2_ActivateAbility`
  (bind _returnvalue (`Actor.GetActorForwardVector` (`self.GetAvatarActorFromActorInfo`)))
  (bind _returnvalue_2 (`self.K2_CommitAbility`))
  (if _returnvalue_2
    (`self.ChangeInputState` false)
    (`AbilityTask_ApplyRootMotionConstantForce.ApplyRootMotionConstantForce` "None" (`KismetMathLibrary.MakeVector` (.x (`KismetMathLibrary.SelectVector` _returnvalue (* _returnvalue -1.0) (`self.Is Moving Forward`))) (.y (`KismetMathLibrary.SelectVector` _returnvalue (* _returnvalue -1.0) (`self.Is Moving Forward`))) (+ (.z (`KismetMathLibrary.SelectVector` _returnvalue (* _returnvalue -1.0) (`self.Is Moving Forward`))) (`self.EvadeHeightStrength`))) (`self.EvadeStrength`) (`self.EvadeDuration`) false (`self.StrengthOverTime`) "MaintainLastRootMotionVelocity"
      (:`then`
        (`AbilityTask_PlayMontageAndWait.CreatePlayMontageAndWaitProxy` "None" (select `bool` (`self.Is Moving Forward`) :`false` (`self.AM_EvadeBackward`) :`true` (`self.AM_EvadeForward`))
          (:`OnCompleted`
            _)
          (:`OnBlendOut`
            _)
          (:`OnInterrupted`
            _)
          (:`OnCancelled`
            _))
        (`self.ChangeInputState` true)
        (`self.K2_EndAbility`)))
    (else
      (`self.K2_EndAbility`))))

(fn `ChangeInputState`
  (params (InputEnabled :type Boolean))
  (bind _aspawn (cast `Pawn` (`self.GetAvatarActorFromActorInfo`)))
  (bind _asplayer_controller (cast `PlayerController` (`Pawn.GetController` _aspawn)))
  (if InputEnabled
    (`Actor.EnableInput` _asplayer_controller _asplayer_controller)
    (else
      (`Actor.DisableInput` _asplayer_controller _asplayer_controller))))

(fn `Is Moving Forward`
  (returns (MovingForward :type Boolean))
  (locals (ErrorTolerance :type "Float (double-precision)" :default 0.2))
  (bind _returnvalue (`self.GetAvatarActorFromActorInfo`))
  (`/Engine/EditorBlueprintResources/StandardMacros.IsValid` _returnvalue
    (:`Is Valid`
      (if (`KismetMathLibrary.NearlyEqual_FloatFloat` (`KismetMathLibrary.Dot_VectorVector` (`Actor.GetActorForwardVector` _returnvalue) (`KismetMathLibrary.Normal` (`Actor.GetVelocity` _returnvalue))) 1.0 (`local.ErrorTolerance`))
        (return true)
        (else
          _)))
    (:`Is Not Valid`
      _))
  (return false))

(fn `K2_CanActivateAbility`
  (params (ActorInfo :type "GameplayAbilityActorInfo Structure") (Handle :type "GameplayAbilitySpecHandle Structure"))
  (returns (RelevantTags :type "GameplayTagContainer Structure") (ReturnValue :type Boolean))
  (bind (_ascharacter_movement_component _bsuccess) (cast `CharacterMovementComponent` ActorInfo_MovementComponent :!pure true))
  (return (struct) (and (`KismetSystemLibrary.IsValid` ActorInfo_AvatarActor) (not (`NavMovementComponent.IsFalling` _ascharacter_movement_component)) _bsuccess)))