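; BP_ChangeMapBoard is an interactable map-selection board that lets the locally controlled server player, in effect the host, use a map widget.
; On overlap it blends the camera to the board and enables the cursor with game-and-UI input, restoring both on exit.
; Widget changes update MapBoardData, whose RepNotify applies the scroll offset and selected map text to the widget, mirroring the board for other players.
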(event `self.ReceiveBeginPlay`
  ;[1 1 1] Begin Play
  (`parent.ReceiveBeginPlay`)
  (bind _aswbp_set_map (cast `/Game/SessionShot/UI/Interaction/LevelSelection/WBP_SetMap` (`WidgetComponent.GetWidget` (`self.WidgetToInteract`))))
  (bind _output_get (set `self.SetMapWidget` _aswbp_set_map))
  (`/Engine/EditorBlueprintResources/StandardMacros.IsValid` _output_get
    (:`Is Valid`
      (add `/Game/SessionShot/UI/Interaction/LevelSelection/WBP_SetMap.OnMapBoardDataChanged` _output_get (delegate `OnMapBoardDataChanged_Event`)))))

(event `OnMapBoardDataChanged_Event`
  (params (NewMapBoardData :type "/Game/SessionShot/Data/Maps/BS_ChangeMapBoardData Structure"))
  ;[1 1 1] Begin Play
  (set `self.MapBoardData` NewMapBoardData))

(event `self.InteractibleCollision.OnComponentBeginOverlap`
  (params (OverlappedComponent :type "PrimitiveComponent Object Reference") (OtherActor :type "Actor Object Reference") (OtherComp :type "PrimitiveComponent Object Reference") (OtherBodyIndex :type Integer) (bFromSweep :type Boolean) (SweepResult :type "HitResult Structure (by ref)"))
  (bind _playercontroller (`self.PlayerController`))
  ;[1 1 1] Begin Overlap
  (if (and (`GameplayStatics.ObjectIsA` OtherActor (`self.PlayerClass`)) (`self.HasAuthority` OtherActor))
    (bind _aspawn (cast `Pawn` OtherActor))
    (bind _output_get (set `self.PlayerPawn` _aspawn))
    (if (`Pawn.IsLocallyControlled` _output_get)
      (bind _output_get_2 (set `self.PlayerController` (`self.Get Player Controller` _output_get)))
      (`/Engine/EditorBlueprintResources/StandardMacros.IsValid` _output_get_2
        (:`Is Valid`
          (`PlayerController.SetViewTargetWithBlend` _output_get_2 self (`self.CameraBlendTime`) "VTBlend_Linear" 0.0 false)
          (set `PlayerController.bShowMouseCursor` true _playercontroller)
          (`WidgetBlueprintLibrary.SetInputMode_GameAndUIEx` _playercontroller null "DoNotLock" false))))))

(event `self.InteractibleCollision.OnComponentEndOverlap`
  (params (OverlappedComponent :type "PrimitiveComponent Object Reference") (OtherActor :type "Actor Object Reference") (OtherComp :type "PrimitiveComponent Object Reference") (OtherBodyIndex :type Integer))
  (if (and (`GameplayStatics.ObjectIsA` OtherActor (`self.PlayerClass`)) (`self.HasAuthority` OtherActor))
    (bind _aspawn (cast `Pawn` OtherActor))
    (bind _output_get (set `self.PlayerController` (`self.Get Player Controller` _aspawn)))
    (`/Engine/EditorBlueprintResources/StandardMacros.IsValid` _output_get
      (:`Is Valid`
        (`PlayerController.SetViewTargetWithBlend` _output_get (`Controller.K2_GetPawn` _output_get) (`self.CameraBlendTime`) "VTBlend_Linear" 0.0 false)
        (set `PlayerController.bShowMouseCursor` false (`self.PlayerController`))
        (`WidgetBlueprintLibrary.SetInputMode_GameOnly` (`self.PlayerController`))))))

(fn `Get Player Controller`
  (params (PlayerPawn :type "Pawn Object Reference"))
  (returns (`AsPlayer Controller` :type "PlayerController Object Reference"))
  (bind _asplayer_controller (cast `PlayerController` (`Pawn.GetController` PlayerPawn))
    (:`then`
      (return _asplayer_controller))
    (:`CastFailed`
      (return null))))

(fn `OnRep_MapBoardData`
  (bind (_mapboarddata_scrollboxoffset _mapboarddata_selectedmaptext) (break `/Game/SessionShot/Data/Maps/BS_ChangeMapBoardData` (`self.MapBoardData`)))
  (bind _mapboarddata_scrollboxoffset_2 (break `/Game/SessionShot/Data/Maps/BS_ChangeMapBoardData` (`self.MapBoardData`)))
  (bind _mapsscrollbox (`/Game/SessionShot/UI/Interaction/LevelSelection/WBP_SetMap.MapsScrollBox` (`self.SetMapWidget`)))
  (bind _tb_mapdescription (`/Game/SessionShot/UI/Interaction/LevelSelection/WBP_SetMap.TB_MapDescription` (`self.SetMapWidget`)))
  (`/Engine/EditorBlueprintResources/StandardMacros.IsValid` (`self.SetMapWidget`)
    (:`Is Valid`
      (`/Engine/EditorBlueprintResources/StandardMacros.IsValid` _mapsscrollbox
        (:`Is Valid`
          (`ScrollBox.SetScrollOffset` _mapsscrollbox _mapboarddata_scrollboxoffset_2))
        (:`Is Not Valid`
          _))
      (`/Engine/EditorBlueprintResources/StandardMacros.IsValid` _tb_mapdescription
        (:`Is Valid`
          (`TextBlock.SetText` _tb_mapdescription (`KismetTextLibrary.Conv_StringToText` _mapboarddata_selectedmaptext)))))))

(fn `UserConstructionScript`
  (`parent.UserConstructionScript`))