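; BP_TestSeamless is a trigger-box actor that, judging by its name, tests seamless travel to the game map.
; When a BaseCharacter with a local player controller begins overlapping the box, it casts the game state to BP_BaseGameState.
; If the cast succeeds, it calls a non-absolute ServerTravel to the map returned by that game state's GetGameMap.
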(event `self.Box.OnComponentBeginOverlap`
  (params (OverlappedComponent :type "PrimitiveComponent Object Reference") (OtherActor :type "Actor Object Reference") (OtherComp :type "PrimitiveComponent Object Reference") (OtherBodyIndex :type Integer) (bFromSweep :type Boolean) (SweepResult :type "HitResult Structure (by ref)"))
  (bind _returnvalue (`Pawn.GetController` (cast `Pawn` OtherActor :!pure true)))
  (bind (_asbp_base_game_state _bsuccess) (cast `/Game/SessionShot/Logic/BP_BaseGameState` (`GameplayStatics.GetGameState`) :!pure true))
  (if (`GameplayStatics.ObjectIsA` OtherActor "/Script/SessionShot.BaseCharacter")
    (`/Engine/EditorBlueprintResources/StandardMacros.IsValid` _returnvalue
      (:`Is Valid`
        (if (`Controller.IsLocalPlayerController` _returnvalue)
          (if _bsuccess
            (`AdvancedSessionsLibrary.ServerTravel` (`BaseGameState.GetGameMap` _asbp_base_game_state))))))))

(fn `UserConstructionScript`)